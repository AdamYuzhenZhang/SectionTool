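; BP_ClippingPlaneVolume is a volume actor with an orthographic scene capture, apparently supporting a clipping plane effect.
; Construction and BeginPlay scale the capture's ortho width by the largest world-scale axis of SphereVolume and store it as BoundingValue.
; BeginPlay also scales the spring arm length the same way and, if AutoSpawnUMG is set, adds the UMG_ClippingPlane widget to the viewport.
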(event `self.ReceiveBeginPlay`
  (bind _returnvalue (`KismetMathLibrary.GetMaxElement` (`SceneComponent.K2_GetComponentScale` (`self.SphereVolume`))))
  (bind _output_get (set `SceneCaptureComponent2D.OrthoWidth` (* 72 _returnvalue) (`self.SceneCaptureComponent2D`)))
  (set `self.BoundingValue` _output_get)
  (set `SpringArmComponent.TargetArmLength` (* 30 _returnvalue) (`self.SpringArm`))
  (if (`self.AutoSpawnUMG`)
    (bind _returnvalue_2 (`|CreateWidget` "/SectionTool/UMG/UMG_ClippingPlane.UMG_ClippingPlane_C" (`GameplayStatics.GetPlayerController` 0)))
    (`UserWidget.AddToViewport` _returnvalue_2 0)))

(fn `UserConstructionScript`
  (bind _output_get (set `SceneCaptureComponent2D.OrthoWidth` (* 72 (`KismetMathLibrary.GetMaxElement` (`SceneComponent.K2_GetComponentScale` (`self.SphereVolume`)))) (`self.SceneCaptureComponent2D`)))
  (set `self.BoundingValue` _output_get))