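; BP_ClippingPlane is an actor that drives a material clipping plane from the transform of its Plane component.
; It writes the component's world location and up vector into the Position and Normal vectors of the MP_ClippingPlane material parameter collection.
; The Construction Script performs this update, and a Clipping event repeats it on demand, with no per-frame Tick update.
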(event `Clipping`
  (bind _plane (`self.Plane`))
  ;[1 1 1] Clipping
  (`KismetMaterialLibrary.SetVectorParameterValue` "/SectionTool/Materials/MP_ClippingPlane.MP_ClippingPlane" "Position" (`KismetMathLibrary.Conv_VectorToLinearColor` (`SceneComponent.K2_GetComponentLocation` _plane)))
  (`KismetMaterialLibrary.SetVectorParameterValue` "/SectionTool/Materials/MP_ClippingPlane.MP_ClippingPlane" "Normal" (`KismetMathLibrary.Conv_VectorToLinearColor` (`SceneComponent.GetUpVector` _plane))))

(fn `UserConstructionScript`
  (bind _plane (`self.Plane`))
  (`KismetMaterialLibrary.SetVectorParameterValue` "/SectionTool/Materials/MP_ClippingPlane.MP_ClippingPlane" "Position" (`KismetMathLibrary.Conv_VectorToLinearColor` (`SceneComponent.K2_GetComponentLocation` _plane)))
  (`KismetMaterialLibrary.SetVectorParameterValue` "/SectionTool/Materials/MP_ClippingPlane.MP_ClippingPlane" "Normal" (`KismetMathLibrary.Conv_VectorToLinearColor` (`SceneComponent.GetUpVector` _plane))))